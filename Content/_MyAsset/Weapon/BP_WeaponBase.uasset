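; BP_WeaponBase is a weapon base Blueprint with a start/stop fire interface and a prototype hitscan shot.
; StartFire calls Fire once, while StopFire is an empty stub.
; Fire prints a debug message, casts player 0's character to BP_Player and traces the Visibility channel forward from its FollowCamera, with debug drawing.
; The trace result is unused, so no hit or damage logic runs.
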(event EventBeginPlay)

(fn ConstructionScript)

(fn StartFire
  (CallFunction|Fire))

(fn StopFire)

(fn Fire
  (Development|PrintString "Fire" true true "(R=1.000000,G=0.000000,B=0.291373,A=1.000000)")
  (bind _asbp_player (Utilities|Casting|CastToBP_Player (Game|GetPlayerCharacter 0)))
  (Collision|LineTraceByChannel (Transformation|GetWorldLocation (Variables|/Game/_MyAsset/System/BP_Player.BP_Player_C|GetFollowCamera _asbp_player)) (+ (Transformation|GetWorldLocation (Variables|/Game/_MyAsset/System/BP_Player.BP_Player_C|GetFollowCamera _asbp_player)) (* (Math|Vector|GetForwardVector (Variables|/Game/_MyAsset/System/BP_Player.BP_Player_C|GetFollowCamera _asbp_player)) 1e+04)) "TraceTypeQuery1" false 0 "ForDuration"))